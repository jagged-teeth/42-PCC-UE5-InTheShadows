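; Player character Blueprint that adds head bobbing and footstep audio.
; Each tick starts a walk or idle camera shake based on velocity and CanJump.
; Tick also plays or stops FootstepTimeline with movement; its Footstep track calls TryFootstep.
; TryFootstep plays a concrete footstep sound when a downward capsule-radius sphere trace hits, without checking surface type.
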(event `Footstep`
  (bind _footsteptimeline (`self.FootstepTimeline`))
  (if (> (`KismetMathLibrary.VSize` (`self.GetVelocity`)) 0.0)
    (`TimelineComponent.Play` _footsteptimeline)
    (else
      (`TimelineComponent.Stop` _footsteptimeline))))

(event `self.ReceiveTick`
  (params (DeltaSeconds :type "Float (single-precision)"))
  (`|ExecutionSequence`
    (:`then_0`
      (`self.HeadBobbing`))
    (:`then_1`
      (`self.Footstep`))))

(event `HeadBobbing`
  (bind _returnvalue (`GameplayStatics.GetPlayerController` 0))
  ;[1 1 1] HeadBobbing
  (if (and (> (`KismetMathLibrary.VSize` (`self.GetVelocity`)) 0.0) (`self.CanJump`))
    (`PlayerController.ClientStartCameraShake` :`self` _returnvalue :`Shake` "/Game/Blueprints/Actors/BP_HeadBobbing_Walk.BP_HeadBobbing_Walk_C")
    (else
      (`PlayerController.ClientStartCameraShake` :`self` _returnvalue :`Shake` "/Game/Blueprints/Actors/BP_HeadBobbing_Idle.BP_HeadBobbing_Idle_C"))))

(fn `FootstepTrace`
  (returns (Sucess :type Boolean))
  (bind _returnvalue (`self.K2_GetActorLocation`))
  (bind _capsulecomponent (`self.CapsuleComponent`))
  (bind (_outhit _returnvalue_2) (`KismetSystemLibrary.SphereTraceSingle` _returnvalue (`KismetMathLibrary.MakeVector` (.x _returnvalue) (.y _returnvalue) (- (.z _returnvalue) (`CapsuleComponent.GetScaledCapsuleHalfHeight` _capsulecomponent))) (`CapsuleComponent.GetScaledCapsuleRadius` _capsulecomponent) "TraceTypeQuery1"))
  (return _returnvalue_2))

(fn `TryFootstep`
  (bind _sucess (`self.FootstepTrace`))
  (if _sucess
    (`GameplayStatics.PlaySoundAtLocation` "/Game/Imports/LiveSound/Footsteps_Concrete_Cue.Footsteps_Concrete_Cue" (`self.K2_GetActorLocation`) (struct) 1.0 1.0 0.0 null null null null)))

(fn `UserConstructionScript`)
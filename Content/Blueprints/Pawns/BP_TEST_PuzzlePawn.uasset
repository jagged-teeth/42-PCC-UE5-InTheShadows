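; BP_TEST_PuzzlePawn is a test puzzle pawn that handles camera transitions to and from the player character.
; On possession, it snaps PuzzleCamera to the player's FollowCamera, then eases it to a fixed relative offset with MoveComponentTo.
; On unpossession, gated by IsUnposs, it moves FollowCamera to the puzzle camera's position and eases it back.
; Snapping one camera onto the other before easing makes the view switch look continuous.
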(event `self.ReceivePossessed`
  (params (NewController :type "Controller Object Reference"))
  (bind _playerref (`self.PlayerRef`))
  (bind _puzzlecamera (`self.PuzzleCamera`))
  (bind _followcamera (`PlayerCharacter.FollowCamera` _playerref))
  (bind (_returnvalue_location _returnvalue_rotation) (`KismetMathLibrary.BreakTransform` (`SceneComponent.K2_GetComponentToWorld` _followcamera)))
  ;[1 1 1 0.372] Camera Transition In
  (if (`KismetSystemLibrary.IsValid` _playerref)
    (if (`KismetSystemLibrary.IsValid` _followcamera)
      (`SceneComponent.K2_SetWorldTransform` _puzzlecamera (`KismetMathLibrary.MakeTransform` _returnvalue_location _returnvalue_rotation) false false)
      (`KismetSystemLibrary.MoveComponentTo` _puzzlecamera (-60.0 0.0 0.0) (struct) true true 0.8 true))))

(event `self.ReceiveUnpossessed`
  (params (OldController :type "Controller Object Reference"))
  (bind _playerref (`self.PlayerRef`))
  (bind (_returnvalue_location _returnvalue_rotation) (`KismetMathLibrary.BreakTransform` (`SceneComponent.K2_GetComponentToWorld` (`self.PuzzleCamera`))))
  (bind _followcamera (`PlayerCharacter.FollowCamera` _playerref))
  ;[1 1 1 0.372] Camera Transition Out
  (if (`self.bIsUnposs`)
    (if (`KismetSystemLibrary.IsValid` _playerref)
      (if (`KismetSystemLibrary.IsValid` _followcamera)
        (`SceneComponent.K2_SetWorldTransform` _followcamera (`KismetMathLibrary.MakeTransform` _returnvalue_location _returnvalue_rotation) false false)
        (`KismetSystemLibrary.MoveComponentTo` _followcamera (0.0 0.0 0.0) (struct) true true 0.8 true)))))

(fn `UserConstructionScript`)
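; BP_PuzzlePawnFirst is the possessable pawn for the game's first puzzle, handling its camera transitions and solved response.
; On possess and unpossess, it blends between the player's follow camera and PuzzleCamera by snapping one to the other, then easing with MoveComponentTo.
; Solve events destroy WallFirst, rotate the mesh to its target on a timeline, play completion sound and delayed voice line, and write the teapot achievement.
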(event `self.DestroyWall`
  (bind _wallfirst (`self.WallFirst`))
  ;[1 1 1] On Solved
  (if (`KismetSystemLibrary.IsValid` _wallfirst)
    (`self.K2_DestroyActor` _wallfirst)))

(event `self.PlayPuzzleSolvedSound`
  (bind _returnvalue (`GameplayStatics.GetPlayerController` 0))
  ;[1 1 1] On Solved
  (`|ExecutionSequence`
    (:`then_0`
      (bind (_direction _alpha) (`Timeline|Timeline_0`)
        (:`Update`
          (`SceneComponent.K2_SetRelativeRotation` (`self.StaticMesh`) (`KismetMathLibrary.RLerp` (`SceneComponent.RelativeRotation` (`self.StaticMesh`)) (`self.GetTargetRotation`) _alpha) false false))))
    (:`then_1`
      (`GameplayStatics.PlaySound2D` "/Game/Imports/LiveSound/Puzzle/PuzzleCompleted_Fixed.PuzzleCompleted_Fixed" 0.3 1.0 0.0 null null)
      (`KismetSystemLibrary.Delay` 0.7)
      (`/Engine/EditorBlueprintResources/StandardMacros.DoOnce` false
        (:`Completed`
          (`GameplayStatics.PlaySound2D` "/Game/Imports/LiveSound/Voice/voices_fixed/voice_firstpuzzle.voice_firstpuzzle" 0.8 1.0 0.0 null null)
          (`AchievementQueryCallbackProxy.CacheAchievements` _returnvalue
            (:`OnSuccess`
              (`AchievementWriteCallbackProxy.WriteAchievementProgress` _returnvalue "ACH_TEAPOT"))))))))

(event `self.ReceivePossessed`
  (params (NewController :type "Controller Object Reference"))
  (bind _playerref (`self.PlayerRef`))
  (bind _puzzlecamera (`self.PuzzleCamera`))
  (bind _followcamera (`PlayerCharacter.FollowCamera` _playerref))
  (bind (_returnvalue_location _returnvalue_rotation) (`KismetMathLibrary.BreakTransform` (`SceneComponent.K2_GetComponentToWorld` _followcamera)))
  ;[1 1 1 0.372] Camera Transition In
  (if (`KismetSystemLibrary.IsValid` _playerref)
    (if (`KismetSystemLibrary.IsValid` _followcamera)
      (`SceneComponent.K2_SetWorldTransform` _puzzlecamera (`KismetMathLibrary.MakeTransform` _returnvalue_location _returnvalue_rotation) false false)
      (`KismetSystemLibrary.MoveComponentTo` _puzzlecamera (-60.0 0.0 0.0) (struct) true true 0.8 true))))

(event `self.ReceiveUnpossessed`
  (params (OldController :type "Controller Object Reference"))
  (bind _playerref (`self.PlayerRef`))
  (bind (_returnvalue_location _returnvalue_rotation) (`KismetMathLibrary.BreakTransform` (`SceneComponent.K2_GetComponentToWorld` (`self.PuzzleCamera`))))
  (bind _followcamera (`PlayerCharacter.FollowCamera` _playerref))
  ;[1 1 1 0.372] Camera Transition Out
  (if (`self.bIsUnposs`)
    (if (`KismetSystemLibrary.IsValid` _playerref)
      (if (`KismetSystemLibrary.IsValid` _followcamera)
        (`SceneComponent.K2_SetWorldTransform` _followcamera (`KismetMathLibrary.MakeTransform` _returnvalue_location _returnvalue_rotation) false false)
        (`KismetSystemLibrary.MoveComponentTo` _followcamera (0.0 0.0 0.0) (struct) true true 0.8 true)))))

(fn `UserConstructionScript`)